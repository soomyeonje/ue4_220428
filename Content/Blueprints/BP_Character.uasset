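; BP_Character is a player-controlled character Blueprint that handles basic movement, jumping and a hold-to-speed-up key.
; MoveForward and MoveRight axis inputs add movement along the control rotation's forward and right vectors, scaled by a Speed variable.
; Holding Tab raises Speed and releasing it lowers it, changing the input scale rather than the movement component's max walk speed.
; The Jump action calls the built-in Jump.
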(event EventBeginPlay)

(event Collision|EventActorBeginOverlap
  (params (OtherActor :type Actor%20Object%20Reference)))

(event EventTick
  (params (DeltaSeconds :type Float%20%28single-precision%29)))

(event Input|ActionEvents|InputActionJump
  (params (Key :type Key%20Structure :default "None"))
  ;[1 1 1] 캐릭터 이동
  (:Pressed
    (Character|Jump)))

(event Input|AxisEvents|InputAxisMoveForward
  (params (AxisValue :type Float%20%28single-precision%29))
  ;[1 1 1] 캐릭터 이동
  (Pawn|Input|AddMovementInput (Math|Vector|GetForwardVector (Pawn|GetControlRotation :!class /Script/Engine.Pawn)) (* AxisValue (Variables|디폴트|GetSpeed)) false))

(event Input|AxisEvents|InputAxisMoveRight
  (params (AxisValue :type Float%20%28single-precision%29))
  ;[1 1 1] 캐릭터 이동
  (Pawn|Input|AddMovementInput (Math|Vector|GetRightVector (Pawn|GetControlRotation :!class /Script/Engine.Pawn)) (* AxisValue (Variables|디폴트|GetSpeed)) false))

(event Input|KeyboardEvents|Tab
  (params (Key :type Key%20Structure :default "None"))
  ;[1 1 1] 캐릭터 이동
  (:Pressed
    (Variables|디폴트|SetSpeed 0.7))
  (:Released
    (Variables|디폴트|SetSpeed 0.5)))

(fn ConstructionScript)